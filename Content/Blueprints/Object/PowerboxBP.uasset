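; Powerbox interactable that the player activates by holding interact (EActive) inside its trigger zone.
; Tick plays or reverses a lever timeline, whose updates rotate the lever and drive a lights timeline.
; That timeline lights three lamps in sequence through dynamic material emissivity and reverses on release until fully activated.
; On first completed activation, it notifies MenuLevelGM through PowerboxActivated.
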(event OnComponentBeginOverlap(TriggerZone)
  (params (OverlappedComponent :type Primitive%20Component%20Object%20Reference) (OtherActor :type Actor%20Object%20Reference) (OtherComp :type Primitive%20Component%20Object%20Reference) (OtherBodyIndex :type Integer) (bFromSweep :type Boolean) (SweepResult :type Hit%20Result%20Structure%20%28by%20ref%29))
  ;[1 1 1] Player in activation zone
  (bind _astop_down_character (Utilities|Casting|CastToTopDownCharacter OtherActor))
  (Variables|Default|SetIn_zone true)
  (Variables|Default|SetPlayer _astop_down_character))

(event OnComponentEndOverlap(TriggerZone)
  (params (OverlappedComponent :type Primitive%20Component%20Object%20Reference) (OtherActor :type Actor%20Object%20Reference) (OtherComp :type Primitive%20Component%20Object%20Reference) (OtherBodyIndex :type Integer))
  ;[1 1 1] Player in activation zone
  (Utilities|Casting|CastToTopDownCharacter OtherActor)
  (Variables|Default|SetIn_zone false))

(event EventTick
  (params (DeltaSeconds :type Float%20%28single-precision%29))
  (bind _lamp_mat_1 (Variables|Default|GetLamp_mat_1))
  (bind _lamp_mat_2 (Variables|Default|GetLamp_mat_2))
  (bind _lamp_mat_3 (Variables|Default|GetLamp_mat_3))
  (if (Variables|Default|GetIn_zone)
    (if (Variables|/Game/Blueprints/Character/TopDownCharacter.TopDownCharacter_C|GetE%20Active (Variables|Default|GetPlayer))
      ;[1 1 1] Lever movement
      (bind _lever_animation (Timeline|Lever_Timeline Play)
        (:Update
          (Transformation|SetWorldRotation (Variables|Default|GetLever) (Math|Rotator|MakeRotator 0.0 (* _lever_animation 1.8e+02) 0.0) false false)
          (if (or (Variables|Default|GetActivated) (Variables|/Game/Blueprints/Character/TopDownCharacter.TopDownCharacter_C|GetE%20Active (Variables|Default|GetPlayer)))
            ;[1 1 1] Lights turning on and off
            (bind _lights (Timeline|Lever%20Lights Play)
              (:Update
                (if (>= _lights 1.0)
                  (Variables|Default|SetActivated true)
                  (else
                    (if (> _lights 0.33)
                      (Rendering|Material|SetScalarParameterValue _lamp_mat_1 "Emisivity" 5.0 :!class /Script/Engine.MaterialInstanceDynamic)
                      (else
                        (Rendering|Material|SetScalarParameterValue _lamp_mat_1 "Emisivity" 0.0 :!class /Script/Engine.MaterialInstanceDynamic)))
                    (if (> _lights 0.66)
                      (Rendering|Material|SetScalarParameterValue _lamp_mat_2 "Emisivity" 5.0 :!class /Script/Engine.MaterialInstanceDynamic)
                      (else
                        (Rendering|Material|SetScalarParameterValue _lamp_mat_2 "Emisivity" 0.0 :!class /Script/Engine.MaterialInstanceDynamic)))
                    (if (> _lights 0.99)
                      (Rendering|Material|SetScalarParameterValue _lamp_mat_3 "Emisivity" 5.0 :!class /Script/Engine.MaterialInstanceDynamic)
                      (else
                        (Rendering|Material|SetScalarParameterValue _lamp_mat_3 "Emisivity" 0.0 :!class /Script/Engine.MaterialInstanceDynamic))))))
              (:Finished
                ;[1 1 1] Letting GM notice about activation
                (if (and (Variables|Default|GetFirst_Time_Actived) (Variables|Default|GetActivated))
                  (bind _asmenu_level_gm (Utilities|Casting|CastToMenuLevelGM (Game|GetGameMode)))
                  (Default|PowerboxActivated _asmenu_level_gm self)
                  (Variables|Default|SetFirst_Time_Actived false))))
            (else
              (Timeline|Lever%20Lights Reverse)))))
      (else
        (Timeline|Lever_Timeline Reverse)))))

(fn ConstructionScript
  (bind _returnvalue (Rendering|Material|CreateDynamicMaterialInstance (Variables|Default|GetLamp_1) 0 0 "None" :!class /Script/Engine.PrimitiveComponent))
  (Variables|Default|SetLamp_mat_1 _returnvalue)
  (bind _returnvalue_2 (Rendering|Material|CreateDynamicMaterialInstance (Variables|Default|GetLamp_2) 0 0 "None" :!class /Script/Engine.PrimitiveComponent))
  (Variables|Default|SetLamp_mat_2 _returnvalue_2)
  (bind _returnvalue_3 (Rendering|Material|CreateDynamicMaterialInstance (Variables|Default|GetLamp_3) 0 0 "None" :!class /Script/Engine.PrimitiveComponent))
  (Variables|Default|SetLamp_mat_3 _returnvalue_3))