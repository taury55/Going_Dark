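; ZoneBP is a join zone for the menu level that tracks characters inside its box and shows progress through a dynamic decal material.
; Each tick plays the infill timeline while players are present and reverses it when empty, unless the zone is deactivated.
; When the fill value drops below a small threshold, it passes its tag and first player to MenuLevelGM, removes that player and restarts the timeline.
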(event OnComponentBeginOverlap(Box)
  (params (OverlappedComponent :type Primitive%20Component%20Object%20Reference) (OtherActor :type Actor%20Object%20Reference) (OtherComp :type Primitive%20Component%20Object%20Reference) (OtherBodyIndex :type Integer) (bFromSweep :type Boolean) (SweepResult :type Hit%20Result%20Structure%20%28by%20ref%29))
  (bind _ascharacter (Utilities|Casting|CastToCharacter OtherActor))
  (Utilities|Array|Add (Variables|Default|GetPlayers) _ascharacter))

(event OnComponentEndOverlap(Box)
  (params (OverlappedComponent :type Primitive%20Component%20Object%20Reference) (OtherActor :type Actor%20Object%20Reference) (OtherComp :type Primitive%20Component%20Object%20Reference) (OtherBodyIndex :type Integer))
  (bind _ascharacter (Utilities|Casting|CastToCharacter OtherActor))
  (Utilities|Array|RemoveItem (Variables|Default|GetPlayers) _ascharacter))

(event EventTick
  (params (DeltaSeconds :type Float%20%28single-precision%29))
  (bind _players (Variables|Default|GetPlayers))
  (Math|Float|CompareFloat (Variables|Default|GetInfill_Value) 0.01
    (:>
      (if (Variables|Default|GetDeactivated) :!label _label
        (bind _newtrack_0 (Timeline|InfillTimeline Stop)
          (:Update
            (bind _output_get (Variables|Default|SetInfill_Value _newtrack_0))
            (Rendering|Material|SetScalarParameterValue (Variables|Default|GetInfillMaterial) "Fill_Amount" _output_get :!class /Script/Engine.MaterialInstanceDynamic)))
        (elif (> (Utilities|Array|Length (Variables|Default|GetPlayers)) 0)
          (Timeline|InfillTimeline Play)
          (else
            (Timeline|InfillTimeline Reverse)))))
    (:==
      (goto _label))
    (:<
      (Variables|Default|SetInfill_Value 1.0)
      (Default|JoinZoneActivated (Variables|Default|GetMenu%20Level%20GM) (Utilities|Array|Get(acopy) (Variables|Actor|GetTags self)) (Utilities|Array|Get(acopy) _players) self)
      (Utilities|Array|RemoveIndex _players)
      (Timeline|InfillTimeline PlayFromStart))))

(event EventBeginPlay
  (bind _asmenu_level_gm (Utilities|Casting|CastToMenuLevelGM (Game|GetGameMode)))
  (Variables|Default|SetMenu%20Level%20GM _asmenu_level_gm))

(fn ConstructionScript
  (bind _returnvalue (Rendering|Material|CreateDynamicMaterialInstance "/Game/Assets/Images/ZoneOutlineInfillMaterialInstance.ZoneOutlineInfillMaterialInstance" "None" "None" :!class /Script/Engine.KismetMaterialLibrary))
  (bind _output_get (Variables|Default|SetInfillMaterial _returnvalue))
  (Rendering|Components|Decal|SetDecalMaterial (Variables|Default|GetZoneOutlineInfillDecal) _output_get))