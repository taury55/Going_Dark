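; Exit gate actor with two sliding doors and a warning alarm.
; Each tick, the Open flag, not set in this graph, plays or reverses a timeline that slides the doors apart along Y.
; Any overlap with the trigger box switches the alarm on and ending overlap switches it off, independently of the doors.
; Tick constantly spins two alarm lights and applies the alarm state to their visibility and a dynamic material's emissive parameter.
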(event OnComponentBeginOverlap(Box)
  (params (OverlappedComponent :type Primitive%20Component%20Object%20Reference) (OtherActor :type Actor%20Object%20Reference) (OtherComp :type Primitive%20Component%20Object%20Reference) (OtherBodyIndex :type Integer) (bFromSweep :type Boolean) (SweepResult :type Hit%20Result%20Structure%20%28by%20ref%29))
  (Variables|Default|SetAlarm true))

(event OnComponentEndOverlap(Box)
  (params (OverlappedComponent :type Primitive%20Component%20Object%20Reference) (OtherActor :type Actor%20Object%20Reference) (OtherComp :type Primitive%20Component%20Object%20Reference) (OtherBodyIndex :type Integer))
  (Variables|Default|SetAlarm false))

(event EventBeginPlay
  (bind _returnvalue (Rendering|Material|CreateDynamicMaterialInstance (Variables|Default|GetMainBody) 1 "/Game/Assets/Geometry/Materials/Gate_Light_Inst.Gate_Light_Inst" "None" :!class /Script/Engine.PrimitiveComponent))
  (Variables|Default|SetAlarm_Material _returnvalue))

(event EventTick
  (params (DeltaSeconds :type Float%20%28single-precision%29))
  (CallFunction|AlarmRotator DeltaSeconds)
  (CallFunction|AlarmVisibility)
  (if (Variables|Default|GetOpen)
    (bind _door_animation (Timeline|Door_Timeline Play)
      (:Update
        (CallFunction|DoorAnimation _door_animation)))
    (else
      (Timeline|Door_Timeline Reverse))))

(fn ConstructionScript
  (Variables|Default|SetDoor_R_Def_Location (Transformation|GetWorldLocation (Variables|Default|GetR_Door)))
  (Variables|Default|SetDoor_L_Def_Location (Transformation|GetWorldLocation (Variables|Default|GetL_Door))))

(fn AlarmRotator
  (params (Value :type Float%20%28single-precision%29%20%28by%20ref%29))
  (bind _result (Math|Float|IncrementFloat Value)
    (:%20%20
      (Transformation|AddLocalRotation (Variables|Default|GetAlarm_LightB) (Math|Rotator|MakeRotator 0.0 (* _result (Variables|Default|GetAlarm_Rotation_Speed)) 0.0) false false)
      (Transformation|AddLocalRotation (Variables|Default|GetAlarm_LightA) (Math|Rotator|MakeRotator 0.0 (* _result (Variables|Default|GetAlarm_Rotation_Speed)) 0.0) false false))))

(fn AlarmVisibility
  (bind _alarm_material (Variables|Default|GetAlarm_Material))
  (bind _alarm (Variables|Default|GetAlarm))
  (if _alarm
    (Rendering|Material|SetScalarParameterValue _alarm_material "Emisivity" 1.0 :!class /Script/Engine.MaterialInstanceDynamic)
    (else
      (Rendering|Material|SetScalarParameterValue _alarm_material "Emisivity" 0.0 :!class /Script/Engine.MaterialInstanceDynamic)))
  (Rendering|SetVisibility (Variables|Default|GetAlarm_LightA) _alarm false)
  (Rendering|SetVisibility (Variables|Default|GetAlarm_LightB) _alarm false)
  (return))

(fn DoorAnimation
  (params (A :type Float%20%28single-precision%29))
  (bind _door_movement (Variables|Default|GetDoor_Movement))
  (bind _returnvalue (* A _door_movement))
  (Transformation|SetRelativeLocation (Variables|Default|GetL_Door) (Math|Vector|MakeVector 0.0 _returnvalue 0.0) false false)
  (Transformation|SetRelativeLocation (Variables|Default|GetR_Door) (Math|Vector|MakeVector 0.0 (* _returnvalue -1.0) 0.0) false false))