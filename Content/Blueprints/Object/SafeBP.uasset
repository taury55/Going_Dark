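; Lockpickable safe that holds a random three-digit combination and pays out coins when opened.
; BeginPlay rolls the three digits, and the trigger zone tells an overlapping ThiefCharacter1 when it enters or leaves lockpick range, passing itself as the target safe.
; OpenSafe swings the door by a yaw offset, spawns FloatingCoinsBP in front of the safe and marks it opened.
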(event OnComponentBeginOverlap(TriggerZone)
  (params (OverlappedComponent :type Primitive%20Component%20Object%20Reference) (OtherActor :type Actor%20Object%20Reference) (OtherComp :type Primitive%20Component%20Object%20Reference) (OtherBodyIndex :type Integer) (bFromSweep :type Boolean) (SweepResult :type Hit%20Result%20Structure%20%28by%20ref%29))
  (bind _asthief_character_1 (Utilities|Casting|CastToThiefCharacter1 OtherActor))
  (Default|IsinLockpickZone _asthief_character_1 true self))

(event OnComponentEndOverlap(TriggerZone)
  (params (OverlappedComponent :type Primitive%20Component%20Object%20Reference) (OtherActor :type Actor%20Object%20Reference) (OtherComp :type Primitive%20Component%20Object%20Reference) (OtherBodyIndex :type Integer))
  (bind _asthief_character_1 (Utilities|Casting|CastToThiefCharacter1 OtherActor))
  (Default|IsinLockpickZone _asthief_character_1 false self))

(event EventBeginPlay
  (bind _returnvalue (Math|Random|RandomIntegerinRange 0 9))
  (Variables|Default|SetNumber_1 _returnvalue)
  (Variables|Default|SetNumber_2 _returnvalue)
  (Variables|Default|SetNumber_3 _returnvalue))

(fn ConstructionScript)

(fn OpenSafe
  (bind _self self)
  (bind _safedoor (Variables|Default|GetSafeDoor))
  (bind _returnvalue (Transformation|GetWorldRotation _safedoor))
  (bind (_roll _pitch _yaw) (Math|Rotator|BreakRotator _returnvalue))
  (Transformation|SetWorldRotation _safedoor (Math|Rotator|MakeRotator _roll _pitch (+ _yaw (Variables|Default|GetDoorRotationAngle))) false false)
  (Game|SpawnActorfromClass "/Game/Blueprints/Object/FloatingCoinsBP.FloatingCoinsBP_C" (Math|Conversions|ToTransform(Vector) (+ (Transformation|GetActorLocation _self) (* (Transformation|GetActorForwardVector _self) (Variables|Default|GetMoneySpawnDistance)))) "Undefined" 0 0)
  (Variables|Default|SetOpened true))