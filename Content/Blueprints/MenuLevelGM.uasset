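; Menu-level game mode that turns session hosting, quick join and team choice into in-world interactions, spawning the first local player as police at the "Start" player start.
; Tagged join zones either run an Advanced Sessions search, calling join on every result, or record a police/thief pick and respawn the character in place as that class.
; A powerbox tagged "HostLobby" hosts a session through GoingDark_Instance.
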(event Custom|JoinZoneActivated
  (params (Tag :type Name) (Player%20Character :type Character%20Object%20Reference) (Zone :type Zone%20BP%20Object%20Reference))
  (bind _returnvalue (Pawn|GetController Player%20Character))
  (bind _returnvalue_2 (Transformation|GetActorTransform Player%20Character))
  (if (Utilities|Name|Equal(Name) Tag "QuickJoin")
    ;[1 1 1] Session Quick Join
    (Development|PrintString "finding")
    (bind _asplayer_controller (Utilities|Casting|CastToPlayerController (Pawn|GetController Player%20Character)))
    (Variables|/Game/Blueprints/Object/ZoneBP.ZoneBP_C|SetDeactivated Zone true)
    (bind _results (|FindSessionsAdvanced _asplayer_controller 999 false "AllServers" 0 false true false 1)
      (:OnSuccess
        (Development|PrintString "found")
        (for _array_element _results
          (Development|PrintString (Class|FindSessionsCallbackProxy|GetServerName _array_element)))
        (Development|PrintString (Utilities|String|ToString(Integer) (Utilities|Array|Length _results)))
        (for _array_element_2 _results
          (Development|PrintString "joining")
          (Default|JoinSession (Variables|Default|GetGame%20Instance) _array_element_2))
        (Variables|/Game/Blueprints/Object/ZoneBP.ZoneBP_C|SetDeactivated Zone false)))
    (else
      ;[1 1 1] Changing teams
      (if (Utilities|Name|Equal(Name) Tag "TeamPoliceJoin")
        (Utilities|Array|Add (Variables|Default|GetPolicePlayers) Player%20Character)
        (CallFunction|Respawn 0 Player%20Character _returnvalue_2 _returnvalue)
        (elif (Utilities|Name|Equal(Name) Tag "TeamThiefJoin")
          (Utilities|Array|Add (Variables|Default|GetThiefPlayers) Player%20Character)
          (CallFunction|Respawn 1 Player%20Character _returnvalue_2 _returnvalue))))))

(event Custom|Powerbox%20Activated
  (params (powerbox :type Powerbox%20BP%20Object%20Reference))
  (if (Utilities|Name|Equal(Name) (Utilities|Array|Get(acopy) (Variables|/Script/Engine.Actor|GetTags powerbox)) "HostLobby")
    (Default|HostSession (Variables|Default|GetGame%20Instance))))

(event EventBeginPlay
  ;[1 1 1] Initial Start
  (CallFunction|GetPlayerStartPoints)
  (CallFunction|SpawnPlayers)
  (bind _asgoing_dark_instance (Utilities|Casting|CastToGoingDark_Instance (Game|GetGameInstance)))
  (Variables|Default|SetGame%20Instance _asgoing_dark_instance))

(fn ConstructionScript)

(fn GetPlayerStartPoints
  (bind _outactors (Actor|GetAllActorsOfClass "/Script/Engine.PlayerStart"))
  (for _array_element _outactors
    (if (Utilities|Name|Equal(Name) (Variables|/Script/Engine.PlayerStart|GetPlayerStartTag _array_element) "Lobby")
      (Variables|Default|SetStart%20Point%20-%20Lobby _array_element)
      (elif (Utilities|Name|Equal(Name) (Variables|/Script/Engine.PlayerStart|GetPlayerStartTag _array_element) "Start")
        (Variables|Default|SetStart%20Point%20-%20Start _array_element)))))

(fn SpawnPlayers
  (for _index (range 0 (- (Variables|Default|GetMaxPlayers) 1))
    (bind _output_get (Variables|Default|SetIndex _index))
    (if (== _output_get 0)
      (Class|GameplayStatics|CreatePlayer (Variables|Default|GetIndex))
      (Game|SpawnActorfromClass "/Game/Blueprints/Character/PoliceCharacter.PoliceCharacter_C" (Transformation|GetActorTransform (Variables|Default|GetStart%20Point%20-%20Start)) "Undefined" 0 0)
      (Pawn|Possess (Game|GetPlayerController (Variables|Default|GetIndex)))
      (Utilities|Array|AddUnique (Variables|Default|GetPlayers) 0))))

(fn Respawn
  (params (Character%20Index :type Integer) (Actor%20To%20Destroy :type Actor%20Object%20Reference) (Spawn%20Location :type Transform) (Controller :type Controller%20Object%20Reference))
  (Actor|DestroyActor Actor%20To%20Destroy)
  (bind _returnvalue (Game|SpawnActorfromClass (Utilities|Select :Index Character%20Index :Option%200 "/Game/Blueprints/Character/PoliceCharacter.PoliceCharacter_C" :Option%201 "/Game/Blueprints/Character/ThiefCharacter1.ThiefCharacter1_C") Spawn%20Location "AdjustIfPossibleButAlwaysSpawn" Controller 0))
  (bind _ascharacter (Utilities|Casting|CastToCharacter _returnvalue))
  (Pawn|Possess Controller _ascharacter))