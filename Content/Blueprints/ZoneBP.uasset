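; Capture-style zone actor that fills a decal while a Pawn stands inside its box and flags itself activated when the fill is nearly full.
; Box overlap events set PlayerInZone, and Tick uses it to play or reverse InfillTimeline, which drives InfillValue and the Fill_Amount parameter of a dynamic decal material created in the construction script.
; Tick also derives ActivatedZone from InfillValue, so it clears when the fill drops.
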(event OnComponentBeginOverlap(Box)
  (params (OverlappedComponent :type Primitive%20Component%20Object%20Reference) (OtherActor :type Actor%20Object%20Reference) (OtherComp :type Primitive%20Component%20Object%20Reference) (OtherBodyIndex :type Integer) (bFromSweep :type Boolean) (SweepResult :type Hit%20Result%20Structure%20%28by%20ref%29))
  (Utilities|Casting|CastToPawn OtherActor)
  (Variables|Default|SetPlayer_In_Zone true))

(event OnComponentEndOverlap(Box)
  (params (OverlappedComponent :type Primitive%20Component%20Object%20Reference) (OtherActor :type Actor%20Object%20Reference) (OtherComp :type Primitive%20Component%20Object%20Reference) (OtherBodyIndex :type Integer))
  (Utilities|Casting|CastToPawn OtherActor)
  (Variables|Default|SetPlayer_In_Zone false))

(event EventTick
  (params (DeltaSeconds :type Float%20%28single-precision%29))
  (Math|Float|CompareFloat (Variables|Default|GetInfill_Value) 0.95
    (:>
      (Variables|Default|SetActivated_Zone true))
    (:==
      (Variables|Default|SetActivated_Zone false :!label _label))
    (:<
      (goto _label)))
  (if (Variables|Default|GetPlayer_In_Zone)
    (bind _newtrack_0 (Timeline|InfillTimeline Play)
      (:Update
        (bind _output_get (Variables|Default|SetInfill_Value _newtrack_0))
        (Rendering|Material|SetScalarParameterValue (Variables|Default|GetInfillMaterial) "Fill_Amount" _output_get :!class /Script/Engine.MaterialInstanceDynamic)))
    (else
      (Timeline|InfillTimeline Reverse))))

(fn ConstructionScript
  (bind _returnvalue (Rendering|Material|CreateDynamicMaterialInstance "/Game/Assets/Images/ZoneOutlineInfillMaterialInstance.ZoneOutlineInfillMaterialInstance" "None" :!class /Script/Engine.KismetMaterialLibrary))
  (bind _output_get (Variables|Default|SetInfillMaterial _returnvalue))
  (Rendering|Components|Decal|SetDecalMaterial (Variables|Default|GetZoneOutlineInfillDecal) _output_get))