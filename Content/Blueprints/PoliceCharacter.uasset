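; Player-controlled police character for top-down cursor-aimed shooting, moving on fixed world axes and turning its controller yaw toward the point under the mouse.
; Firing spends ammo and spawns a projectile from a forward-right offset with a pistol sound; muzzle flash is an empty stub and empty-gun sound has no asset.
; A looping timer regenerates ammo, while Tick updates three bullet indicators and line-traces to position the laser-sight beam.
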(event EventBeginPlay
  (Utilities|Time|SetTimerbyFunctionName 0 "GettingAmmo" (Variables|Default|GetReloadSpeed) true))

(event EventTick
  (params (DeltaSeconds :type Float%20%28single-precision%29))
  (bind _self self)
  (bind _laserps (Variables|Default|GetLaserPS))
  (bind _returnvalue (Transformation|GetActorLocation _self))
  (bind _returnvalue_2 (Transformation|GetActorForwardVector _self))
  (bind _returnvalue_3 (Transformation|GetActorRightVector _self))
  (bind _returnvalue_4 (* _returnvalue_3 65.0))
  (CallFunction|AmmoBarUpdate)
  (bind (_outhit _returnvalue_5) (Collision|LineTraceByChannel (+ _returnvalue (+ (* _returnvalue_2 1e+02) _returnvalue_4)) (+ (+ (* _returnvalue_2 8e+03) _returnvalue_4) _returnvalue) "TraceTypeQuery1" false 0 "None"))
  (if _returnvalue_5
    (Class|ParticleSystemComponent|SetBeamSourcePoint _laserps 0 (.TraceStart (Collision|BreakHitResult _outhit)))
    (Class|ParticleSystemComponent|SetBeamTargetPoint _laserps 0 (.ImpactPoint (Collision|BreakHitResult _outhit)))))

(event Input|ActionEvents|InputActionFirePrimaryWeapon
  (params (Key :type Key%20Structure :default "None"))
  (:Pressed
    (bind _can_fire (CallFunction|CanFire))
    (if _can_fire
      (CallFunction|DecrementAmmoCount)
      (CallFunction|PlayMuzzleFlash)
      (CallFunction|PlayFireSound)
      (CallFunction|FireProjectile)
      (else
        (CallFunction|PlayEmptyGunSound)))))

(event Input|AxisEvents|InputAxisMoveForward
  (params (AxisValue :type Float%20%28single-precision%29))
  (Pawn|Input|AddMovementInput "90.000000,0.000000, 0" AxisValue false)
  (CallFunction|RotateFacetoCursor))

(event Input|AxisEvents|InputAxisMoveRight
  (params (AxisValue :type Float%20%28single-precision%29))
  (Pawn|Input|AddMovementInput "0,90.000000, 0" AxisValue false)
  (CallFunction|RotateFacetoCursor))

(fn ConstructionScript)

(fn RotateFacetoCursor
  (bind _returnvalue (Game|GetPlayerController 0))
  (Pawn|SetControlRotation _returnvalue (Math|Rotator|MakeRotator 0.0 0.0 (.yaw (Math|Rotator|FindLookatRotation (Transformation|GetActorLocation self) (.Location (Collision|BreakHitResult (.HitResult (Game|Player|GetHitResultUnderCursorbyChannel _returnvalue "TraceTypeQuery1" true)))))))))

(fn FireProjectile
  (bind _self self)
  (Game|SpawnActorfromClass "/Game/Blueprints/Projectile.Projectile_C" (Math|Transform|MakeTransform (+ (Transformation|GetActorLocation _self) (+ (* (Transformation|GetActorForwardVector _self) 1e+02) (* (Transformation|GetActorRightVector _self) 65.0))) (Transformation|GetActorRotation _self) "0.200000,0.100000,0.200000") "Undefined" self (Game|GetInstigator)))

(fn CanFire
  (return (> (Variables|Default|GetAmmoCount) 0.0)))

(fn DecrementAmmoCount
  (Variables|Default|SetAmmoCount (Math|Float|Clamp(Float) (- (Variables|Default|GetAmmoCount) 1.0) 0.0 (Variables|Default|GetMaxAmmo))))

(fn PlayMuzzleFlash)

(fn PlayFireSound
  (Audio|PlaySoundatLocation "/Game/Assets/Audio/PistolShot.PistolShot" (Transformation|GetActorLocation self) "0, 0, 0" 1.0 1.0 0.0 0 0 0))

(fn PlayEmptyGunSound
  (Audio|PlaySoundatLocation 0 (Transformation|GetActorLocation self) "0, 0, 0" 1.0 1.0 0.0 0 0 0))

(fn GettingAmmo
  (if (< (Variables|Default|GetAmmoCount) (Variables|Default|GetMaxAmmo))
    (Variables|Default|SetAmmoCount (+ (Variables|Default|GetAmmoCount) 1.0))))

(fn AmmoBarUpdate
  (bind _ammocount (Variables|Default|GetAmmoCount))
  (Rendering|SetVisibility (Variables|Default|GetBullet1) (> _ammocount 0.0) false)
  (Rendering|SetVisibility (Variables|Default|GetBullet2) (> _ammocount 1.0) false)
  (Rendering|SetVisibility (Variables|Default|GetBullet3) (> _ammocount 2.0) false))