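; FloatingCoinsBP is a coin pickup that spins and bobs in place, granting money to the thief character that touches it.
; Tick advances the capsule's yaw by a mostly frame-based step and derives height from the absolute sine of that yaw, bouncing it above its BeginPlay height.
; On overlap, any ThiefCharacter1 other than the coin's owner receives MoneyAmount through AddMoney, then the coin destroys itself.
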(event EventBeginPlay
  (Variables|Default|SetZ_Origin (.Z (Math|Vector|BreakVector (Transformation|GetWorldLocation (Variables|Default|GetCapsule))))))

(event EventTick
  (params (DeltaSeconds :type Float%20%28single-precision%29))
  (bind _capsule (Variables|Default|GetCapsule))
  (bind _returnvalue (Transformation|GetWorldLocation _capsule))
  (bind _returnvalue_2 (Transformation|GetWorldRotation _capsule))
  (bind (_x _y) (Math|Vector|BreakVector _returnvalue))
  (bind (_roll _pitch _yaw) (Math|Rotator|BreakRotator _returnvalue_2))
  (bind _result (Math|Float|IncrementFloat DeltaSeconds)
    (:%20%20
      (Transformation|SetWorldLocationAndRotation _capsule (Math|Vector|MakeVector _x _y (+ (Variables|Default|GetZ_Origin) (Math|Float|Absolute(Float) (* (Variables|Default|GetFloatingAmplitude) (Math|Trig|Sin(Degrees) (* (Variables|Default|GetFloatingSpeed) _yaw)))))) (Math|Rotator|MakeRotator _roll _pitch (+ (* _result 1.0) _yaw)) false false))))

(event Collision|EventActorBeginOverlap
  (params (OtherActor :type Actor%20Object%20Reference))
  (bind _asthief_character_1 (Utilities|Casting|CastToThiefCharacter1 OtherActor))
  (if (not (== _asthief_character_1 (Components|GetOwner)))
    (Default|AddMoney _asthief_character_1 (Variables|Default|GetMoneyAmount))
    (Actor|DestroyActor)))

(fn ConstructionScript)