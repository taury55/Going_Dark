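; Floating coin actor that spins and bobs its Coins component every Tick.
; Yaw grows by the incremented DeltaSeconds each frame, so spin speed depends on frame rate.
; That yaw, scaled by FloatingSpeed, drives an absolute sine times FloatingAmplitude for height.
; The result sets world Z directly rather than offsetting from the placed height, while X and Y stay unchanged.
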(event EventBeginPlay)

(event Collision|EventActorBeginOverlap
  (params (OtherActor :type Actor%20Object%20Reference)))

(event EventTick
  (params (DeltaSeconds :type Float%20%28single-precision%29))
  (bind _coins (Variables|Default|GetCoins))
  (bind _returnvalue (Transformation|GetWorldLocation _coins))
  (bind _returnvalue_2 (Transformation|GetWorldRotation _coins))
  (bind (_x _y) (Math|Vector|BreakVector _returnvalue))
  (bind (_roll _pitch _yaw) (Math|Rotator|BreakRotator _returnvalue_2))
  (bind _result (Math|Float|IncrementFloat DeltaSeconds)
    (:%20%20
      (Transformation|SetWorldLocationAndRotation _coins (Math|Vector|MakeVector _x _y (Math|Float|Absolute(Float) (* (Variables|Default|GetFloatingAmplitude) (Math|Trig|Sin(Degrees) (* (Variables|Default|GetFloatingSpeed) _yaw))))) (Math|Rotator|MakeRotator _roll _pitch (+ (* _result 1.0) _yaw)) false false))))

(fn ConstructionScript)