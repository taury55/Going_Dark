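; Thief character Blueprint that carries money, takes damage and unlocks safes.
; When health runs out, it spawns a floating coins actor holding its money amount, then destroys itself.
; Pressing the primary action finds an overlapping, unopened safe through an interface check, shows the unlock widget and messages the safe.
; Releasing the action removes the widget; the lockpick-zone function is an empty stub.
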(event Custom|End%20Unlocking
  ;[1 1 1] Safe interaction
  ;;[1 1 1] Ending unlocking
  (Widget|RemovefromParent (Variables|Default|GetSafe%20Widget)))

(event Game|Damage|EventAnyDamage
  (params (Damage :type Float%20%28single-precision%29) (DamageType :type Damage%20Type%20Object%20Reference) (InstigatedBy :type Controller%20Object%20Reference) (DamageCauser :type Actor%20Object%20Reference))
  (bind _self self)
  ;[1 1 1] Health and death
  (Variables|Default|SetHealth (- (Variables|Default|GetHealth) Damage))
  (if (<= (Variables|Default|GetHealth) 0.0)
    (bind _returnvalue (Game|SpawnActorfromClass "/Game/Blueprints/Object/FloatingCoinsBP.FloatingCoinsBP_C" (Math|Conversions|ToTransform(Vector) (Transformation|GetActorLocation _self)) "Undefined" _self 0))
    (Variables|/Game/Blueprints/Object/FloatingCoinsBP.FloatingCoinsBP_C|SetMoneyAmount _returnvalue (Variables|Default|GetMoneyAmount))
    (Actor|DestroyActor)))

(event Input|ActionEvents|InputActionPrimaryActionBtn
  (params (Key :type Key%20Structure :default "None"))
  ;[1 1 1] Safe interaction
  (:Pressed
    (bind _array_element (Utilities|Array|ForEachLoopwithBreak (Collision|GetOverlappingActors 0 :!class /Script/Engine.Actor) :!label _label)
      (:LoopBody
        (if (Utilities|DoesObjectImplementInterface _array_element "/Game/Blueprints/Object/BPi_safe.BPi_safe_C")
          (bind _assafe_bp (Utilities|Casting|CastToSafeBP _array_element))
          (if (not (Variables|/Game/Blueprints/Object/SafeBP.SafeBP_C|GetOpened _assafe_bp))
            (Variables|Default|SetSafe _assafe_bp)
            (CallFunction|AddUnlockWidget)
            (Class|BPiSafe|UnlockingInteraction(Message) _array_element self)
            (goto _label Break))))))
  (:Released
    (CallFunction|EndUnlocking)))

(fn ConstructionScript)

(fn AddMoney
  (params (MoneyAmount :type Float%20%28single-precision%29))
  (Variables|Default|SetMoneyAmount (+ MoneyAmount (Variables|Default|GetMoneyAmount))))

(fn IsinLockpickZone
  (params (ThiefInZone :type Boolean) (SafeObject :type Actor%20Object%20Reference)))

(fn AddUnlockWidget
  (bind _returnvalue (UserInterface|CreateWidget "/Game/Blueprints/Widget/SafeWidget.SafeWidget_C"))
  (bind _output_get (Variables|Default|SetSafe%20Widget _returnvalue))
  (UserInterface|Viewport|AddtoViewport _output_get 0)
  (return _output_get))