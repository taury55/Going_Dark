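; Player thief character for a top-down game that moves on world axes, turns to face the cursor, carries money and cracks safes.
; Holding the primary button in a safe's zone shows the lock widget and debug-prints the combination.
; E checks the widget's three numbers in order against the safe, opening it on success or resetting on a miss.
; Lethal damage spawns floating coins holding its money, then destroys it.
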(event Game|Damage|EventAnyDamage
  (params (Damage :type Float%20%28single-precision%29) (DamageType :type Damage%20Type%20Object%20Reference) (InstigatedBy :type Controller%20Object%20Reference) (DamageCauser :type Actor%20Object%20Reference))
  (bind _self self)
  (Variables|Default|SetHealth (- (Variables|Default|GetHealth) Damage))
  (if (<= (Variables|Default|GetHealth) 0.0)
    (bind _returnvalue (Game|SpawnActorfromClass "/Game/Blueprints/Object/FloatingCoinsBP.FloatingCoinsBP_C" (Math|Conversions|ToTransform(Vector) (Transformation|GetActorLocation _self)) "Undefined" _self 0))
    (Variables|/Game/Blueprints/Object/FloatingCoinsBP.FloatingCoinsBP_C|SetMoneyAmount _returnvalue (Variables|Default|GetMoneyAmount))
    (Actor|DestroyActor)))

(event Input|ActionEvents|InputActionPrimaryActionBtn
  (params (Key :type Key%20Structure :default "None"))
  (:Pressed
    (if (Variables|Default|GetInLockpickZone)
      (bind _assafe_bp (Utilities|Casting|CastToSafeBP (Variables|Default|GetSafe)))
      (if (not (Variables|/Game/Blueprints/Object/SafeBP.SafeBP_C|GetOpened _assafe_bp))
        (CallFunction|AddUnlockWidget)
        ;[1 1 1] Until sound for unlocking will be added
        (bind _assafe_bp_2 (Utilities|Casting|CastToSafeBP (Variables|Default|GetSafe)))
        (Development|PrintString (Utilities|String|ToString(Integer) (Variables|/Game/Blueprints/Object/SafeBP.SafeBP_C|GetNumber_1 _assafe_bp_2)))
        (Development|PrintString (Utilities|String|ToString(Integer) (Variables|/Game/Blueprints/Object/SafeBP.SafeBP_C|GetNumber_2 _assafe_bp_2)))
        (Development|PrintString (Utilities|String|ToString(Integer) (Variables|/Game/Blueprints/Object/SafeBP.SafeBP_C|GetNumber_3 _assafe_bp_2))))))
  (:Released
    (Viewport|RemoveAllWidgets)))

(event Input|ActionEvents|InputActionE_Button
  (params (Key :type Key%20Structure :default "None"))
  (:Pressed
    (CallFunction|UnlockingSequence)))

(event Input|AxisEvents|InputAxisMoveForward
  (params (AxisValue :type Float%20%28single-precision%29))
  (Pawn|Input|AddMovementInput "90.000000,0.000000, 0" AxisValue false)
  (CallFunction|RotateFacetoCursor))

(event Input|AxisEvents|InputAxisMoveRight
  (params (AxisValue :type Float%20%28single-precision%29))
  (Pawn|Input|AddMovementInput "0,90.000000, 0" AxisValue false)
  (CallFunction|RotateFacetoCursor))

(fn ConstructionScript)

(fn RotateFacetoCursor
  (bind _returnvalue (Game|GetPlayerController 0))
  (Pawn|SetControlRotation _returnvalue (Math|Rotator|MakeRotator 0.0 0.0 (.yaw (Math|Rotator|FindLookatRotation (Transformation|GetActorLocation self) (.Location (Collision|BreakHitResult (.HitResult (Game|Player|GetHitResultUnderCursorbyChannel _returnvalue "TraceTypeQuery1" true)))))))))

(fn GetCrosshairWorldspace
  (return (.Location (Collision|BreakHitResult (.HitResult (Game|Player|GetHitResultUnderCursorbyChannel (Game|GetPlayerController 0) "TraceTypeQuery1" true))))))

(fn AddMoney
  (params (MoneyAmount :type Float%20%28single-precision%29))
  (Variables|Default|SetMoneyAmount (+ MoneyAmount (Variables|Default|GetMoneyAmount))))

(fn IsinLockpickZone
  (params (ThiefInZone :type Boolean) (SafeObject :type Actor%20Object%20Reference))
  (Variables|Default|SetInLockpickZone ThiefInZone)
  (Variables|Default|SetSafe SafeObject))

(fn AddUnlockWidget
  (bind _returnvalue (UserInterface|CreateWidget "/Game/Blueprints/Widget/SafeWidget.SafeWidget_C"))
  (bind _output_get (Variables|Default|SetSafeWidget _returnvalue))
  (UserInterface|Viewport|AddtoViewport _output_get 0))

(fn ResetDoneNumbers
  (bind _safewidget (Variables|Default|GetSafeWidget))
  (Variables|/Game/Blueprints/Widget/SafeWidget.SafeWidget_C|SetNumber_1_int _safewidget 0)
  (Variables|/Game/Blueprints/Widget/SafeWidget.SafeWidget_C|SetNumber_2_int _safewidget 0)
  (Variables|/Game/Blueprints/Widget/SafeWidget.SafeWidget_C|SetNumber_3_int _safewidget 0)
  (Variables|/Game/Blueprints/Widget/SafeWidget.SafeWidget_C|SetWrong _safewidget true)
  (Variables|Default|SetNumber_1_Done false)
  (Variables|Default|SetNumber_2_Done false)
  (Variables|Default|SetNumber_3_Done false)
  (Variables|Default|SetNumber_Done_Change true))

(fn UnlockingSequence
  (bind _assafe_bp (Utilities|Casting|CastToSafeBP (Variables|Default|GetSafe)))
  (Variables|Default|SetNumber_Done_Change true)
  (if (Variables|Default|GetNumber_1_Done)
    (if (Variables|Default|GetNumber_2_Done)
      (if (== (Variables|/Game/Blueprints/Widget/SafeWidget.SafeWidget_C|GetNumber_3_int (Variables|Default|GetSafeWidget)) (Variables|/Game/Blueprints/Object/SafeBP.SafeBP_C|GetNumber_3 _assafe_bp))
        (Variables|Default|SetNumber_3_Done true)
        (Default|OpenSafe _assafe_bp)
        (Viewport|RemoveAllWidgets)
        (CallFunction|ResetDoneNumbers)
        (else
          (CallFunction|ResetDoneNumbers)))
      (elif (== (Variables|/Game/Blueprints/Widget/SafeWidget.SafeWidget_C|GetNumber_2_int (Variables|Default|GetSafeWidget)) (Variables|/Game/Blueprints/Object/SafeBP.SafeBP_C|GetNumber_2 _assafe_bp))
        (Variables|Default|SetNumber_2_Done true)
        (else
          (CallFunction|ResetDoneNumbers))))
    (elif (== (Variables|/Game/Blueprints/Widget/SafeWidget.SafeWidget_C|GetNumber_1_int (Variables|Default|GetSafeWidget)) (Variables|/Game/Blueprints/Object/SafeBP.SafeBP_C|GetNumber_1 _assafe_bp))
      (Variables|Default|SetNumber_1_Done true)
      (else
        (CallFunction|ResetDoneNumbers)))))