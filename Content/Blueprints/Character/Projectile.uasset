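; Projectile actor that damages the thief character on hit and spawns an impact explosion before destroying itself.
; On begin play, its mesh and sphere ignore the owner when moving.
; A sphere hit applies damage only to ThiefCharacter1; other hits clear HitThief.
; ImpactEffects uses that flag to choose the player or mesh explosion particle; the flag is never set true here, so it relies on its default.
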(event OnComponentHit(Sphere)
  (params (HitComponent :type Primitive%20Component%20Object%20Reference) (OtherActor :type Actor%20Object%20Reference) (OtherComp :type Primitive%20Component%20Object%20Reference) (NormalImpulse :type Vector :default "0, 0, 0") (Hit :type Hit%20Result%20Structure%20%28by%20ref%29))
  (bind _asthief_character_1 (Utilities|Casting|CastToThiefCharacter1 OtherActor)
    (:then
      (Game|Damage|ApplyDamage _asthief_character_1 (Variables|Default|GetDMG) 0 0))
    (:CastFailed
      (Variables|Default|SetHitThief false)))
  (CallFunction|ImpactEffects (Variables|Default|GetHitThief))
  (Actor|DestroyActor))

(event EventBeginPlay
  (bind _returnvalue (Components|GetOwner))
  (Collision|IgnoreActorwhenMoving (Variables|Default|GetMesh) _returnvalue true)
  (Collision|IgnoreActorwhenMoving (Variables|Default|GetSphere) _returnvalue true))

(fn ConstructionScript)

(fn ImpactEffects
  (params (HitThief :type Boolean))
  (bind _self self)
  (bind _returnvalue (Transformation|GetActorLocation _self))
  (if HitThief
    (Effects|SpawnEmitteratLocation "/Game/Assets/VFX/BulletExplosionPlayerPS.BulletExplosionPlayerPS" _returnvalue)
    (else
      (Effects|SpawnEmitteratLocation "/Game/Assets/VFX/BulletExplosionMeshPS.BulletExplosionMeshPS" _returnvalue))))